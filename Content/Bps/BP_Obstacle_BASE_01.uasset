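; Base obstacle Blueprint that snaps itself onto the surface at its location and measures its own length when play begins.
; BeginPlay runs a vertical Visibility line trace through the root and moves the root to the impact point, without checking that the trace hit.
; It then stores ObstacleDistance as the world X difference between its Start and Finish components, a signed value along that axis only.
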(event `self.ReceiveBeginPlay`
  (bind _returnvalue (`SceneComponent.K2_GetComponentLocation` (`self.DefaultSceneRoot`)))
  (bind _returnvalue_x (`KismetMathLibrary.BreakVector` (`SceneComponent.K2_GetComponentLocation` (`self.Start`))))
  (bind _returnvalue_x_2 (`KismetMathLibrary.BreakVector` (`SceneComponent.K2_GetComponentLocation` (`self.Finish`))))
  (bind _outhit (`KismetSystemLibrary.LineTraceSingle` (`KismetMathLibrary.MakeVector` (.x _returnvalue) (.y _returnvalue) (+ (.z _returnvalue) 1000.0)) (`KismetMathLibrary.MakeVector` (.x _returnvalue) (.y _returnvalue) (- (.z _returnvalue) 1000.0)) "TraceTypeQuery1"))
  (`SceneComponent.K2_SetWorldLocation` (`self.DefaultSceneRoot`) (`.ImpactPoint` (`GameplayStatics.BreakHitResult` _outhit)) false false)
  (set `self.ObstacleDistance` (- _returnvalue_x _returnvalue_x_2)))

(fn `UserConstructionScript`)
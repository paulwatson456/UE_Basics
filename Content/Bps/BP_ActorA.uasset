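; BP_ActorA is an interactable light actor that shows a widget while the player is nearby.
; The widget starts hidden and toggles with Box overlap begin and end for actors tagged Player.
; Its Interact event calls LightChange, where a FlipFlop alternates the PointLight intensity between off and bright, switching off on the first use.
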(event `self.ReceiveBeginPlay`
  (`SceneComponent.SetVisibility` (`self.Widget`) false false))

(event `self.Box.OnComponentBeginOverlap`
  (params (OverlappedComponent :type "PrimitiveComponent Object Reference") (OtherActor :type "Actor Object Reference") (OtherComp :type "PrimitiveComponent Object Reference") (OtherBodyIndex :type Integer) (bFromSweep :type Boolean) (SweepResult :type "HitResult Structure (by ref)"))
  (if (`self.ActorHasTag` OtherActor "Player")
    (`SceneComponent.SetVisibility` (`self.Widget`) true false)))

(event `self.Box.OnComponentEndOverlap`
  (params (OverlappedComponent :type "PrimitiveComponent Object Reference") (OtherActor :type "Actor Object Reference") (OtherComp :type "PrimitiveComponent Object Reference") (OtherBodyIndex :type Integer))
  (if (`self.ActorHasTag` OtherActor "Player")
    (`SceneComponent.SetVisibility` (`self.Widget`) false false)))

(event `Interact`
  (`self.LightChange`))

(event `LightChange`
  (`/Engine/EditorBlueprintResources/StandardMacros.FlipFlop`
    (:`A`
      (`LightComponent.SetIntensity` (`self.PointLight`) 0.0))
    (:`B`
      (`LightComponent.SetIntensity` (`self.PointLight`) 10000.0))))

(fn `UserConstructionScript`)
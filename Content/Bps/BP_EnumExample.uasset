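; An example actor that demonstrates switching on a wealth enum.
; On BeginPlay it enables input from the first player controller, and pressing F sets its State to a random enum value by converting a random integer to a byte.
; Tick switches on State every frame and prints a message for Poor, Doing Ok or Super Rich.
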(event `self.ReceiveBeginPlay`
  (`self.EnableInput` (`GameplayStatics.GetPlayerController` 0)))

(event `self.ReceiveTick`
  (params (DeltaSeconds :type "Float (single-precision)"))
  (switch `/Game/eNUMS/E_wealth` (`self.State`)
    (:`NewEnumerator0`
      (`KismetSystemLibrary.PrintString` "Oh no, I am so poor"))
    (:`NewEnumerator1`
      (`KismetSystemLibrary.PrintString` "I am doing ok"))
    (:`NewEnumerator2`
      (`KismetSystemLibrary.PrintString` "Woop"))))

(event `Key|F`
  (params (Key :type "Key Structure"))
  (:`Pressed`
    (set `self.State` (cast `/Game/eNUMS/E_wealth` (`KismetMathLibrary.Conv_IntToByte` (`KismetMathLibrary.RandomInteger` 3))))))

(fn `UserConstructionScript`)
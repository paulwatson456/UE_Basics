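; Procedural track generator that builds a runway from random section actors and extends it as the player advances.
; BeginPlay spawns the first section, then loops to chain more, requesting an obstacle from BP_ObstacleSpawner_01 after each.
; Downward traces at each mesh's forward bounds set the next spawn point, where a box trigger spawns another piece on Player-tagged overlap.
; CullTrack can destroy old pieces but is never called here; debug drawing remains on.
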(event `self.ReceiveBeginPlay`
  (bind (_returnvalue_roll _returnvalue_pitch _returnvalue_yaw) (`KismetMathLibrary.BreakRotator` (`SceneComponent.K2_GetComponentRotation` (`self.Arrow`))))
  (bind _returnvalue (`|SpawnActorFromClass` (`|GetArrayItem` (`self.RunwaySections_01`)) (`KismetMathLibrary.MakeTransform` (`SceneComponent.K2_GetComponentLocation` (`self.DefaultSceneRoot`)) (`KismetMathLibrary.MakeRotator` 0.0 0.0 _returnvalue_yaw)) "Undefined" "OverrideRootScale" null null))
  (set `self.SectionPlacementROT` (`KismetMathLibrary.MakeRotator` _returnvalue_roll _returnvalue_pitch _returnvalue_yaw))
  (set `self.TrackPiece` _returnvalue)
  (bind (_origin _boxextent) (`KismetSystemLibrary.GetComponentBounds` (`/Game/Bps/Procedural/BP_ProcRunwaySectionBASE.StaticMesh` _returnvalue)))
  (bind _returnvalue_2 (+ _origin (* _boxextent (`SceneComponent.GetForwardVector` (`/Game/Bps/Procedural/BP_ProcRunwaySectionBASE.Arrow` _returnvalue)))))
  (bind _outhit (`KismetSystemLibrary.LineTraceSingle` :`Start` (+ _returnvalue_2 (0.0 0.0 1000.0)) :`End` (- _returnvalue_2 (0.0 0.0 2000.0)) :`TraceChannel` "TraceTypeQuery1" :`DrawTime` 20.0))
  (bind _output_get (set `self.SectionPlacementPOS` (`.ImpactPoint` (`GameplayStatics.BreakHitResult` _outhit))))
  (`KismetSystemLibrary.DrawDebugSphere` _output_get 100.0 12 (struct :`R` 1.0 :`G` 1.0 :`B` 1.0 :`A` 1.0) 20.0 10.0)
  (`/Engine/EditorBlueprintResources/StandardMacros.DoOnce` false
    (:`Completed`
      (for _ (range 7)
        (`self.CreateTrackPieces`)
        (`self.obstaclemaker`)))))

(event `CreateTrackPieces`
  (bind (_returnvalue_roll _returnvalue_pitch _returnvalue_yaw) (`KismetMathLibrary.BreakRotator` (`SceneComponent.K2_GetComponentRotation` (`self.Arrow`))))
  (bind _returnvalue (`|SpawnActorFromClass` (`KismetArrayLibrary.Array_Random` (`self.RunwaySections_01`)) (`KismetMathLibrary.MakeTransform` (`self.SectionPlacementPOS`) (`KismetMathLibrary.MakeRotator` 0.0 0.0 _returnvalue_yaw)) "Undefined" "OverrideRootScale" null null))
  (bind _end_point (`self.ClacEndOfMeshBounds` (`/Game/Bps/Procedural/BP_ProcRunwaySectionBASE.StaticMesh` _returnvalue) (`/Game/Bps/Procedural/BP_ProcRunwaySectionBASE.Arrow` _returnvalue)))
  (bind _output_get (set `self.SectionPlacementPOS` (`.ImpactPoint` (`GameplayStatics.BreakHitResult` _end_point))))
  (`KismetSystemLibrary.DrawDebugSphere` _output_get 100.0 12 (struct :`R` 1.0 :`G` 1.0 :`B` 1.0 :`A` 1.0) 20.0 10.0)
  (bind _returnvalue_2 (`AddComponent|NODE_AddBoxComponent-0` :`RelativeTransform` (`KismetMathLibrary.MakeTransform` _output_get (struct) (1.0 25.0 40.0))))
  (add `PrimitiveComponent.OnComponentBeginOverlap` _returnvalue_2 (delegate `OnComponentBeginOverlap_Event_0`)))

(event `OnComponentBeginOverlap_Event_0`
  (params (OverlappedComponent :type "PrimitiveComponent Object Reference") (OtherActor :type "Actor Object Reference") (OtherComp :type "PrimitiveComponent Object Reference") (OtherBodyIndex :type Integer) (bFromSweep :type Boolean) (SweepResult :type "HitResult Structure (by ref)"))
  (if (`self.ActorHasTag` OtherActor "Player")
    (`self.CreateTrackPieces`)))

(event `CullTrack`
  (`self.K2_DestroyActor` (`|GetArrayItem` (`self.TrackList`) (`self.TrackNumber`)))
  (`/Engine/EditorBlueprintResources/StandardMacros.IncrementInt` (`self.TrackNumber`)))

(event `obstaclemaker`
  (bind _returnvalue (`GameplayStatics.GetActorOfClass` "/Game/Bps/BP_ObstacleSpawner_01.BP_ObstacleSpawner_01_C"))
  (`/Game/Bps/BP_ObstacleSpawner_01.SpawnObstacle` _returnvalue (`self.SectionPlacementPOS`) 2000.0))

(fn `ClacEndOfMeshBounds`
  (params (`Static Mesh` :type "SceneComponent Object Reference") (`Forward Vector Component` :type "SceneComponent Object Reference"))
  (returns (`End Point` :type "HitResult Structure"))
  (bind (_origin _boxextent) (`KismetSystemLibrary.GetComponentBounds` `Static Mesh`))
  (bind _returnvalue (+ _origin (* _boxextent (`SceneComponent.GetForwardVector` `Forward Vector Component`))))
  (bind _outhit (`KismetSystemLibrary.BoxTraceSingle` :`Start` (+ _returnvalue (0.0 0.0 1000.0)) :`End` (- _returnvalue (0.0 0.0 1000.0)) :`HalfSize` (1.0 1.0 1.0) :`TraceChannel` "TraceTypeQuery1" :`DrawDebugType` "Persistent"))
  (return _outhit))

(fn `UserConstructionScript`)
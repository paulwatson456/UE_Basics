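; BP_ProcGenerator_BASE is a procedural track generator that builds a runway from chained section actors when play begins.
; It spawns a base section at its own location and arrow yaw, then appends eight sections picked at random from the RunwaySections01 array.
; Each new section attaches at the previous one's EndPoint location and Arrow rotation, so the pieces themselves define the track's path.
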(event `self.ReceiveBeginPlay`
  (bind (_returnvalue_roll _returnvalue_pitch _returnvalue_yaw) (`KismetMathLibrary.BreakRotator` (`SceneComponent.K2_GetComponentRotation` (`self.Arrow`))))
  (bind _returnvalue (`|SpawnActorFromClass` "/Game/Bps/Procedural/BP_ProcRunwaySectionBASE.BP_ProcRunwaySectionBASE_C" (`KismetMathLibrary.MakeTransform` (`SceneComponent.K2_GetComponentLocation` (`self.DefaultSceneRoot`)) (`KismetMathLibrary.MakeRotator` 0.0 0.0 _returnvalue_yaw)) "Undefined" "OverrideRootScale" null null))
  (set `self.SectionPlacementPOS` (`SceneComponent.K2_GetComponentLocation` (`/Game/Bps/Procedural/BP_ProcRunwaySectionBASE.EndPoint` _returnvalue)))
  (set `self.SectionPlacementROT` (`SceneComponent.K2_GetComponentRotation` (`/Game/Bps/Procedural/BP_ProcRunwaySectionBASE.Arrow` _returnvalue)))
  (for _ (range 8)
    (bind _returnvalue_2 (`|SpawnActorFromClass` (`KismetArrayLibrary.Array_Random` (`self.RunwaySections_01`)) (`KismetMathLibrary.MakeTransform` (`self.SectionPlacementPOS`) (`self.SectionPlacementROT`)) "Undefined" "OverrideRootScale" null null))
    (set `self.SectionPlacementPOS` (`SceneComponent.K2_GetComponentLocation` (`/Game/Bps/Procedural/BP_ProcRunwaySectionBASE.EndPoint` _returnvalue_2)))
    (set `self.SectionPlacementROT` (`SceneComponent.K2_GetComponentRotation` (`/Game/Bps/Procedural/BP_ProcRunwaySectionBASE.Arrow` _returnvalue_2)))))

(fn `UserConstructionScript`)
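; Procedural track generator that builds a track from random section actors on BeginPlay.
; It spawns TrackInformation entry 1 at its own position, then chains eight more sections at each previous EndPoint location and Arrow rotation.
; Candidates match InputRoute to the last OutputRoute, but accumulate in a never-cleared array.
; Spawned class and next OutputRoute come from separate Random calls, so they can differ.
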(event `self.ReceiveBeginPlay`
  (bind _outitem (`KismetArrayLibrary.Array_Random` (`self.TrackSectionTobuild`)))
  (bind (_returnvalue_roll _returnvalue_pitch _returnvalue_yaw) (`KismetMathLibrary.BreakRotator` (`SceneComponent.K2_GetComponentRotation` (`self.Arrow`))))
  (bind (_tracksection _inputroute _outputroute) (break `/Game/Bps/Procedural/ST_ProcTrack` (`|GetArrayItem` (`self.TrackInformation`) 1)))
  (set `self.OutputRoute` _outputroute)
  (bind _returnvalue (`|SpawnActorFromClass` _tracksection (`KismetMathLibrary.MakeTransform` (`SceneComponent.K2_GetComponentLocation` (`self.DefaultSceneRoot`)) (`KismetMathLibrary.MakeRotator` 0.0 0.0 _returnvalue_yaw)) "Undefined" "OverrideRootScale" null null))
  (set `self.SectionPlacementPOS` (`SceneComponent.K2_GetComponentLocation` (`/Game/Bps/Procedural/BP_ProcRunwaySectionBASE.EndPoint` _returnvalue)))
  (set `self.SectionPlacementROT` (`SceneComponent.K2_GetComponentRotation` (`/Game/Bps/Procedural/BP_ProcRunwaySectionBASE.Arrow` _returnvalue)))
  (for _ (range 8)
    (for (_array_element _array_index) (`self.TrackInformation`)
      (if (== (`.InputRoute_7_16580FE54F2A54624C4AD8AD7719A603` (break `/Game/Bps/Procedural/ST_ProcTrack` _array_element)) (`self.OutputRoute`))
        (`KismetArrayLibrary.Array_Add` (`self.TrackSectionTobuild`) (`|GetArrayItem` (`self.TrackInformation`) _array_index))))
    (bind _returnvalue_2 (`|SpawnActorFromClass` (break `/Game/Bps/Procedural/ST_ProcTrack` _outitem) (`KismetMathLibrary.MakeTransform` (`self.SectionPlacementPOS`) (`self.SectionPlacementROT`)) "Undefined" "OverrideRootScale" null null))
    (set `self.OutputRoute` (`.OutputRoute_8_1E084EBB440F4E733C03E1BBC536483C` (break `/Game/Bps/Procedural/ST_ProcTrack` _outitem)))
    (set `self.SectionPlacementPOS` (`SceneComponent.K2_GetComponentLocation` (`/Game/Bps/Procedural/BP_ProcRunwaySectionBASE.EndPoint` _returnvalue_2)))
    (set `self.SectionPlacementROT` (`SceneComponent.K2_GetComponentRotation` (`/Game/Bps/Procedural/BP_ProcRunwaySectionBASE.Arrow` _returnvalue_2)))))

(fn `UserConstructionScript`)
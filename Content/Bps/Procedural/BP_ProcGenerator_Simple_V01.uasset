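; Procedural runway generator that builds an endless track from random section actors as the player advances.
; On BeginPlay it spawns the first array section at its own location and Arrow yaw, then pre-builds a short run of random pieces.
; Each piece spawns at the previous EndPoint location and gets a runtime box trigger at its own EndPoint.
; A Player-tagged overlap appends another piece; old pieces are never removed here.
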(event `self.ReceiveBeginPlay`
  (`self.SpawnInitialTrack`))

(event `SpawnInitialTrack`
  (bind (_returnvalue_roll _returnvalue_pitch _returnvalue_yaw) (`KismetMathLibrary.BreakRotator` (`SceneComponent.K2_GetComponentRotation` (`self.Arrow`))))
  ;[1 1 1] Spawns initial track of 6 pieces (through for loop) so that an amount of track can be seen in the distance
  (bind _returnvalue (`|SpawnActorFromClass` (`|GetArrayItem` (`self.RunwaySections_01`)) (`KismetMathLibrary.MakeTransform` (`SceneComponent.K2_GetComponentLocation` (`self.DefaultSceneRoot`)) (`KismetMathLibrary.MakeRotator` 0.0 0.0 _returnvalue_yaw)) "Undefined" "OverrideRootScale" null null))
  (set `self.SectionPlacementPOS` (`SceneComponent.K2_GetComponentLocation` (`/Game/Bps/Procedural/BP_ProcRunwaySectionBASE.EndPoint` _returnvalue)))
  (`/Engine/EditorBlueprintResources/StandardMacros.DoOnce` false
    (:`Completed`
      (for _ (range 7)
        (`self.CreateTrackPieces`)))))

(event `CreateTrackPieces`
  (bind _returnvalue (`|SpawnActorFromClass` (`KismetArrayLibrary.Array_Random` (`self.RunwaySections_01`)) (`KismetMathLibrary.Conv_VectorToTransform` (`self.SectionPlacementPOS`)) "Undefined" "OverrideRootScale" null null))
  (bind _endpoint (`/Game/Bps/Procedural/BP_ProcRunwaySectionBASE.EndPoint` _returnvalue))
  (set `self.SectionPlacementPOS` (`SceneComponent.K2_GetComponentLocation` _endpoint))
  ;[1 1 1] Creates a box trigger at the end point of each track piece to call the creation of another track piece when overlapped by the payer
  (bind _returnvalue_2 (`AddComponent|NODE_AddBoxComponent-1` :`self` _returnvalue :`RelativeTransform` (`KismetMathLibrary.MakeTransform` (`SceneComponent.RelativeLocation` _endpoint) (struct) (1.0 25.0 40.0))))
  (add `PrimitiveComponent.OnComponentBeginOverlap` _returnvalue_2 (delegate `OnComponentBeginOverlap_Event_0`)))

(event `OnComponentBeginOverlap_Event_0`
  (params (OverlappedComponent :type "PrimitiveComponent Object Reference") (OtherActor :type "Actor Object Reference") (OtherComp :type "PrimitiveComponent Object Reference") (OtherBodyIndex :type Integer) (bFromSweep :type Boolean) (SweepResult :type "HitResult Structure (by ref)"))
  ;[1 1 1] Creates a box trigger at the end point of each track piece to call the creation of another track piece when overlapped by the payer
  (if (`self.ActorHasTag` OtherActor "Player")
    (`self.CreateTrackPieces`)))

(fn `UserConstructionScript`)
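; An example actor demonstrating procedural random selection techniques, triggered by key presses and printing results to screen.
; G and H use a random integer to pick one food or a whole food group with equal odds.
; F does weighted picking by testing a random float against each spawn entry's low/high bounds.
; J filters choices by a threshold into a temporary array, prints a random pick, then clears it.
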(event `self.ReceiveBeginPlay`
  (`self.EnableInput` (`GameplayStatics.GetPlayerController` 0)))

(event `Key|G`
  (params (Key :type "Key Structure"))
  ;[1 1 1] Both examples use a random INT to select a variable or even an array of varibales. This means that each variable in the list has an equal chance of being selected.
  (:`Pressed`
    (set `self.RandomInt` (`KismetMathLibrary.RandomIntegerInRange` 0 2))
    (`KismetSystemLibrary.PrintString` (select `int` (`self.RandomInt`) :`0` (`self.Food_01`) :`1` (`self.Food_02`) :`2` (`self.Food_03`)))))

(event `Key|H`
  (params (Key :type "Key Structure"))
  ;[1 1 1] Both examples use a random INT to select a variable or even an array of varibales. This means that each variable in the list has an equal chance of being selected.
  (:`Pressed`
    (set `self.RandomInt` (`KismetMathLibrary.RandomIntegerInRange` 0 2))
    (for _array_element (select `int` (`self.RandomInt`) :`0` (`self.FoodGroups01`) :`1` (`self.FoodGroups02`) :`2` (`self.FoodGroups03`))
      (`KismetSystemLibrary.PrintString` _array_element))))

(event `Key|F`
  (params (Key :type "Key Structure"))
  ;[1 1 1] Weighted choices means that you can define how likely a variable is selected. In this case each item in the array has a low and high boundary to represent the chance of being picked. For example if the difference between the low and high boundary is 0.5, then there is a 50% chance it will be picked. Uses a random float (0-1) to generate the conditional to check against
  (:`Pressed`
    (set `self.RandomFloat` (`KismetMathLibrary.RandomFloatInRange` 0.0 1.0))
    (for _array_element (`self.ObjectsToSpawn`)
      (bind (_tracksection _inputroute _outputroute _weightinglow _weightinghigh _name) (break `/Game/Bps/Procedural/ST_ProcTrack` _array_element))
      (if (`KismetMathLibrary.InRange_FloatFloat` (`self.RandomFloat`) _weightinglow _weightinghigh)
        (`KismetSystemLibrary.PrintString` _name)
        (`KismetSystemLibrary.PrintString` (`KismetStringLibrary.Conv_DoubleToString` (`self.RandomFloat`)))))))

(event `Key|J`
  (params (Key :type "Key Structure"))
  ;[1 1 1] Creates a new array of variables based on a conditional
  (:`Pressed`
    (for _array_element (`self.ListOfChoices`)
      (if (>= _array_element 10)
        (`KismetArrayLibrary.Array_Add` (`self.NewListOfChoicesBasedOnConditional`) _array_element)))
    (`KismetSystemLibrary.PrintString` (`KismetStringLibrary.Conv_IntToString` (`KismetArrayLibrary.Array_Random` (`self.NewListOfChoicesBasedOnConditional`))))
    ;[1 1 1] If you are creating a new list and dont want to keep any previous data added before the next calculation, then you need to "clear" the data from the array before hand.
    (`KismetArrayLibrary.Array_Clear` (`self.NewListOfChoicesBasedOnConditional`))))

(fn `UserConstructionScript`)
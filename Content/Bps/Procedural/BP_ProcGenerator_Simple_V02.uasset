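; Procedural track generator that spawns a chain of random track sections, starting from its own location and arrow yaw.
; BeginPlay places the first TrackInformation entry, then seven random sections, each at the previous EndPoint with the first section's rotation.
; Each new section calls BP_ObstacleSpawner_01 for obstacles; the placement point only advances when that spawner exists.
; CullTrack destroys the oldest tracked section by advancing an index.
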(event `self.ReceiveBeginPlay`
  (bind (_returnvalue_roll _returnvalue_pitch _returnvalue_yaw) (`KismetMathLibrary.BreakRotator` (`SceneComponent.K2_GetComponentRotation` (`self.Arrow`))))
  (bind _returnvalue (`|SpawnActorFromClass` (`.TrackSection_9_7A0CCC3D4EFA4F48D506688FECE5D30B` (break `/Game/Bps/Procedural/ST_ProcTrack` (`|GetArrayItem` (`self.TrackInformation`)))) (`KismetMathLibrary.MakeTransform` (`SceneComponent.K2_GetComponentLocation` (`self.DefaultSceneRoot`)) (`KismetMathLibrary.MakeRotator` 0.0 0.0 _returnvalue_yaw)) "Undefined" "OverrideRootScale" null null))
  (set `self.SectionPlacementPOS` (`SceneComponent.K2_GetComponentLocation` (`/Game/Bps/Procedural/BP_ProcRunwaySectionBASE.EndPoint` _returnvalue)))
  (set `self.SectionPlacementROT` (`SceneComponent.K2_GetComponentRotation` (`/Game/Bps/Procedural/BP_ProcRunwaySectionBASE.Arrow` _returnvalue)))
  (`KismetArrayLibrary.Array_Add` (`self.TrackList`) _returnvalue)
  (`/Engine/EditorBlueprintResources/StandardMacros.DoOnce` false
    (:`Completed`
      (for _ (range 7)
        (`self.CreateTrackPieces`)))))

(event `CreateTrackPieces`
  (bind _sectionplacementpos (`self.SectionPlacementPOS`))
  (bind _returnvalue (`|SpawnActorFromClass` (`.TrackSection_9_7A0CCC3D4EFA4F48D506688FECE5D30B` (break `/Game/Bps/Procedural/ST_ProcTrack` (`KismetArrayLibrary.Array_Random` (`self.TrackInformation`)))) (`KismetMathLibrary.MakeTransform` _sectionplacementpos (`self.SectionPlacementROT`)) "Undefined" "OverrideRootScale" null null))
  (`KismetArrayLibrary.Array_Add` (`self.TrackList`) _returnvalue)
  (bind _returnvalue_2 (`GameplayStatics.GetActorOfClass` "/Game/Bps/BP_ObstacleSpawner_01.BP_ObstacleSpawner_01_C"))
  (`/Engine/EditorBlueprintResources/StandardMacros.IsValid` _returnvalue_2
    (:`Is Valid`
      (`/Game/Bps/BP_ObstacleSpawner_01.SpawnObstacle` _returnvalue_2 _sectionplacementpos 2000.0)
      (set `self.SectionPlacementPOS` (`SceneComponent.K2_GetComponentLocation` (`/Game/Bps/Procedural/BP_ProcRunwaySectionBASE.EndPoint` _returnvalue))))))

(event `CullTrack`
  (`self.K2_DestroyActor` (`|GetArrayItem` (`self.TrackList`) (`self.TrackNumber`)))
  (`/Engine/EditorBlueprintResources/StandardMacros.IncrementInt` (`self.TrackNumber`)))

(fn `UserConstructionScript`)
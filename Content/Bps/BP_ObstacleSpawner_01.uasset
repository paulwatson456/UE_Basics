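; Obstacle spawner that fills a track segment with a chain of randomly chosen obstacle actors.
; SpawnObstacle receives a start position and track distance, then spawns random classes from ObstaclesToSpawn in a capped loop.
; Each obstacle adds its length to a running ObstacleDistance, and its Finish component's world location becomes the next spawn point.
; Spawning stops once that total, never reset here, reaches the track distance.
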(event `self.ReceiveBeginPlay`)

(event `SpawnObstacle`
  (params (TrackPOS :type "Vector Structure") (TrackDistance :type "Float (double-precision)"))
  (bind _output_get (set `self.Track POS` TrackPOS))
  (for _ (range 21)
    (if (>= (`self.ObstacleDistance`) TrackDistance)
      (break)
      (else
        (bind _returnvalue (`|SpawnActorFromClass` (`KismetArrayLibrary.Array_Random` (`self.ObstaclesToSpawn`)) (`KismetMathLibrary.Conv_VectorToTransform` (`KismetMathLibrary.MakeVector` (.x _output_get) (.y _output_get) (.z _output_get))) "Undefined" "OverrideRootScale" null null))
        (set `self.ObstacleDistance` (+ (`/Game/Bps/BP_Obstacle_BASE_01.ObstacleDistance` _returnvalue) (`self.ObstacleDistance`)))
        (set `self.Track POS` (`SceneComponent.K2_GetComponentLocation` (`/Game/Bps/BP_Obstacle_BASE_01.Finish` _returnvalue)))))))

(fn `UserConstructionScript`)
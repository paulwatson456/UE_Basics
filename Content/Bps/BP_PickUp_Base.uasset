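; BP_PickUp_Base is a pickup actor that adds an item to the player's inventory.
; Any actor overlap casts player pawn 0 to BP_ThirdPersonCharacter without checking the overlapping actor, passes ItemName to UpdateInventory, plays a 2D pickup sound and destroys the pickup.
; The construction script switches on Type, giving the Sphere component a cube mesh and offset for the Battery type.
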(event `self.ReceiveActorBeginOverlap`
  (params (OtherActor :type "Actor Object Reference"))
  (bind _asbp_third_person_character (cast `/Game/ThirdPerson/Blueprints/BP_ThirdPersonCharacter` (`GameplayStatics.GetPlayerPawn` 0)))
  (`/Game/ThirdPerson/Blueprints/BP_ThirdPersonCharacter.UpdateInventory` _asbp_third_person_character (`self.ItemName`))
  (`GameplayStatics.PlaySound2D` "/Game/Sounds/332629__treasuresounds__item-pickup.332629__treasuresounds__item-pickup" 1.0 1.0 0.0 null null)
  (`self.K2_DestroyActor`))

(fn `UserConstructionScript`
  (bind _sphere (`self.Sphere`))
  (switch `/Game/eNUMS/E_Pickups` (`self.Type`)
    (:`NewEnumerator1`
      (`StaticMeshComponent.SetStaticMesh` _sphere "/Game/LevelPrototyping/Meshes/SM_Cube.SM_Cube")
      (`SceneComponent.K2_SetRelativeLocation` _sphere (-50.0 -50.0 -50.0) false false))))
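; Interactable door that starts locked and needs a matching key from the player before it can swing open.
; Interact switches on State: while Locked, it searches the ThirdPersonCharacter's PickUps for KeyIdentifier01, then either sets Open or reports the missing key.
; Once unlocked, later interactions use a FlipFlop and MoveComponentTo to rotate DoorPivot open and closed.
; Each outcome plays a 2D sound, and unlock attempts also print a message.
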(event `self.ReceiveBeginPlay`
  (`parent.ReceiveBeginPlay`)
  (set `self.State` "NewEnumerator0"))

(event `self.Interact`
  (switch `/Game/eNUMS/E_Interactable` (`self.State`)
    (:`NewEnumerator0`
      (`self.Unlock`))
    (:`NewEnumerator2`
      (`self.OpenClose`))))

(event `Unlock`
  (bind _keyidentifier_01 (`self.KeyIdentifier_01`))
  (bind _asbp_third_person_character (cast `/Game/ThirdPerson/Blueprints/BP_ThirdPersonCharacter` (`GameplayStatics.GetPlayerPawn` 0)))
  (if (`KismetArrayLibrary.Array_Contains` (`/Game/ThirdPerson/Blueprints/BP_ThirdPersonCharacter.PickUps` _asbp_third_person_character) _keyidentifier_01)
    (`KismetSystemLibrary.PrintString` "You have unlocked the door!")
    (set `self.State` "NewEnumerator2")
    (`GameplayStatics.PlaySound2D` (`self.SoundUnlock`) 1.0 1.0 0.0 null null)
    (else
      (`KismetSystemLibrary.PrintString` (`KismetStringLibrary.Concat_StrStr` "Door locked, you need to find the " _keyidentifier_01))
      (`GameplayStatics.PlaySound2D` (`self.SoundLocked`) 1.0 1.0 0.0 null null))))

(event `OpenClose`
  (bind _doorpivot (`self.DoorPivot`))
  (bind _doorpivot_2 (`self.DoorPivot`))
  (bind (_returnvalue_roll _returnvalue_pitch) (`KismetMathLibrary.BreakRotator` (`SceneComponent.K2_GetComponentRotation` _doorpivot)))
  (bind (_returnvalue_roll_2 _returnvalue_pitch_2) (`KismetMathLibrary.BreakRotator` (`SceneComponent.K2_GetComponentRotation` _doorpivot_2)))
  (`/Engine/EditorBlueprintResources/StandardMacros.FlipFlop`
    (:`A`
      (`GameplayStatics.PlaySound2D` (`self.SoundOpen`) 1.0 1.0 0.0 null null)
      (`KismetSystemLibrary.MoveComponentTo` _doorpivot_2 (`SceneComponent.RelativeLocation` _doorpivot_2) (`KismetMathLibrary.MakeRotator` _returnvalue_roll_2 _returnvalue_pitch_2 -90.0)))
    (:`B`
      (`KismetSystemLibrary.MoveComponentTo` _doorpivot (`SceneComponent.RelativeLocation` _doorpivot) (`KismetMathLibrary.MakeRotator` _returnvalue_roll _returnvalue_pitch))
      (`GameplayStatics.PlaySound2D` (`self.SoundOpen`) 1.0 1.0 0.0 null null))))

(fn `UserConstructionScript`
  (`parent.UserConstructionScript`))
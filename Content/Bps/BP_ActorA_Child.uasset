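; BP_ActorA_Child is a child actor Blueprint that toggles the color of its point light when interacted with.
; Its Interact event runs a FlipFlop that alternates the PointLight between white and green on each call.
; The construction script only calls the parent's, and BeginPlay, overlap and Tick are disabled placeholders.
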(event `self.Interact`
  (`/Engine/EditorBlueprintResources/StandardMacros.FlipFlop`
    (:`A`
      (`LightComponent.SetLightColor` (`self.PointLight`) (make `LinearColor` 1.0 1.0 1.0 1.0) true))
    (:`B`
      (`LightComponent.SetLightColor` (`self.PointLight`) (make `LinearColor` 0.0 1.0 0.0 1.0) true))))

(fn `UserConstructionScript`
  (`parent.UserConstructionScript`))
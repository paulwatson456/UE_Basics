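; Turret Blueprint that patrols, locks onto the player and fires, driven by a three-state switch: Patrol, Scan and Fire, Reset.
; A timeline and MultiGate swing the neck between two waypoint rotations until a tagged player overlaps Vision.
; It then yaw-tracks the player and, after a short delay, repeatedly line-traces, spawning explosion effects at impacts without applying damage.
; Leaving Vision eases the neck back to the first waypoint to resume patrol.
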(event `self.ReceiveBeginPlay`
  ;[1 1 1] Logic to move between states
  (set `self.State` "NewEnumerator0")
  (`self.SetState`)
  (`self.EnableInput` (`GameplayStatics.GetPlayerController` 0)))

(event `Patrol`
  ;[1 1 1] Patrol state logic
  (`|MultiGate` false true :!label _label
    (:`Out 0`
      (bind (_direction _newtrack_0) (`Timeline|PatrolMovement` :!via `PlayFromStart` :!label _label_2)
        (:`Update`
          (`SceneComponent.K2_SetRelativeRotation` (`self.TurretNeck`) (`KismetMathLibrary.RLerp` (`self.Waypoint_01`) (`self.Waypoint_02`) _newtrack_0) false false))
        (:`Finished`
          (`KismetSystemLibrary.Delay` (`self.PauseTime`))
          (`self.Patrol`))))
    (:`Out 1`
      (goto _label_2 :!via `Reverse`))))

(event `ResetPatrol`
  ;[1 1 1] Patrol state logic
  (goto _label :!via `Reset`))

(event `SetState`
  ;[1 1 1] Logic to move between states
  (switch `/Game/eNUMS/E_AI` (`self.State`)
    (:`NewEnumerator0`
      (`self.Patrol`))
    (:`NewEnumerator4`
      (`self.ResetTurretPos`))
    (:`NewEnumerator1`
      (`self.Scan`))))

(event `StopPatrol`
  ;[1 1 1] Patrol state logic
  (goto _label_2 :!via `Stop`))

(event `self.Vision.OnComponentBeginOverlap`
  (params (OverlappedComponent :type "PrimitiveComponent Object Reference") (OtherActor :type "Actor Object Reference") (OtherComp :type "PrimitiveComponent Object Reference") (OtherBodyIndex :type Integer) (bFromSweep :type Boolean) (SweepResult :type "HitResult Structure (by ref)"))
  ;[1 1 1] Logic to move between states
  (if (`self.ActorHasTag` OtherActor "Player")
    (`self.StopPatrol`)
    (`self.StopReset`)
    (set `self.State` "NewEnumerator1")
    (`self.SetState`)
    (set `self.PlayerScanned?` true)))

(event `Scan`
  ;[1 1 1] Scan logic
  (`|ExecutionSequence`
    (:`then_0`
      (`self.TrackPlayer`))
    (:`then_1`
      (`self.CountdownToFire`))))

(event `TrackPlayer`
  ;[1 1 1] Scan logic
  (bind (_direction _newtrack_0) (`Timeline|Track Player` :!via `PlayFromStart` :!label _label_3)
    (:`Update`
      (bind (_returnvalue_roll _returnvalue_pitch _returnvalue_yaw) (`KismetMathLibrary.BreakRotator` (`KismetMathLibrary.RLerp` (`SceneComponent.K2_GetComponentRotation` (`self.TurretNeck`)) (`KismetMathLibrary.FindLookAtRotation` (`SceneComponent.K2_GetComponentLocation` (`self.TurretNeck`)) (`self.K2_GetActorLocation` (`GameplayStatics.GetPlayerPawn` 0))) _newtrack_0 true)))
      (`SceneComponent.K2_SetRelativeRotation` (`self.TurretNeck`) (`KismetMathLibrary.MakeRotator` 0.0 0.0 _returnvalue_yaw) false false))
    (:`Finished`
      (`self.TrackPlayer`))))

(event `self.Vision.OnComponentEndOverlap`
  (params (OverlappedComponent :type "PrimitiveComponent Object Reference") (OtherActor :type "Actor Object Reference") (OtherComp :type "PrimitiveComponent Object Reference") (OtherBodyIndex :type Integer))
  ;[1 1 1] Logic to move between states
  (if (`self.ActorHasTag` OtherActor "Player")
    (set `self.State` "NewEnumerator4")
    (set `self.PlayerScanned?` false)
    (`self.StopTrackingPlayer`)
    (`self.SetState`)))

(event `StopTrackingPlayer`
  ;[1 1 1] Scan logic
  (goto _label_3 :!via `Stop`))

(event `ResetTurretPos`
  (bind _turretneck (`self.TurretNeck`))
  ;[1 1 1] Logic to move between states
  (`KismetSystemLibrary.MoveComponentTo` _turretneck (`SceneComponent.RelativeLocation` _turretneck) (`self.Waypoint_01`) false false 2.0 :!label _label_4)
  (if (not (`self.PlayerScanned?`))
    (set `self.State` "NewEnumerator0")
    (`self.ResetPatrol`)
    (`self.SetState`)))

(event `StopReset`
  ;[1 1 1] Logic to move between states
  (goto _label_4 :!via `Stop`))

(event `CountdownToFire`
  ;[1 1 1] Scan logic
  (`KismetSystemLibrary.Delay` 0.5)
  (`self.Fire`))

(event `Fire`
  ;[1 1 1] Firing logic
  (if (`self.PlayerScanned?`)
    (bind _output_get (set `self.ShootStart` (`SceneComponent.K2_GetComponentLocation` (`self.Arrow`))))
    (bind _outhit (`KismetSystemLibrary.LineTraceSingle` _output_get (`self.K2_GetActorLocation` (`GameplayStatics.GetPlayerPawn` 0)) "TraceTypeQuery2" true))
    (set `self.ShootEnd` (`.ImpactPoint` (`GameplayStatics.BreakHitResult` _outhit)))
    (`NiagaraFunctionLibrary.SpawnSystemAtLocation` "/Game/ThirdPerson/Blueprints/Explosion.Explosion" (`self.ShootEnd`))
    (`KismetSystemLibrary.Delay` 0.2)
    (`self.Fire`)))

(fn `UserConstructionScript`)
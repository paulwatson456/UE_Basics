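; Actor component that creates the in-game HUD widget and tracks counts for three pickup skills.
; AddSkill matches the item name to raise the matching count and refresh its widget display.
; Only skill one has a use path, which spends a charge and fires a debug-drawn forward line trace from the player pawn.
; An explosion effect spawns at the impact point without checking for a hit.
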(event `self.ReceiveBeginPlay`
  (bind _returnvalue (`|CreateWidget` "/Game/Bps/Inventory/W_InGameHUD.W_InGameHUD_C" (`GameplayStatics.GetPlayerController` 0)))
  (bind _output_get (set `self.HUD` _returnvalue))
  (`UserWidget.AddToViewport` _output_get 0))

(event `AddSkill`
  (params (ItemData :type "/Game/Bps/Inventory/ST_Items_01 Structure"))
  (bind (_itemname _itemnumber) (break `/Game/Bps/Inventory/ST_Items_01` ItemData))
  (switch `string` (`KismetStringLibrary.Conv_NameToString` _itemname)
    (:`Skill1`
      (bind _output_get (set `self.SkillOneNumber` (+ (`self.SkillOneNumber`) _itemnumber)))
      (`/Game/Bps/Inventory/W_InGameHUD.SkillOneUpdate` (`self.HUD`) _output_get))
    (:`Skill2`
      (bind _output_get_2 (set `self.SkillTwoNumber` (+ (`self.SkillTwoNumber`) _itemnumber)))
      (`/Game/Bps/Inventory/W_InGameHUD.SkillTwoUpdate` (`self.HUD`) _output_get_2))
    (:`Skill3`
      (bind _output_get_3 (set `self.SkillThreeNumber` (+ (`self.SkillThreeNumber`) _itemnumber)))
      (`/Game/Bps/Inventory/W_InGameHUD.SkillThreeUpdate` (`self.HUD`) _output_get_3))))

(event `UseSkillOne`
  (if (> (`self.SkillOneNumber`) 0)
    (bind _output_get (set `self.SkillOneNumber` (- (`self.SkillOneNumber`) 1)))
    (`/Game/Bps/Inventory/W_InGameHUD.SkillOneUpdate` (`self.HUD`) _output_get)
    (`self.FireSkillOne`)))

(event `FireSkillOne`
  (bind _returnvalue (`GameplayStatics.GetPlayerPawn` 0))
  (bind _returnvalue_2 (`Actor.K2_GetActorLocation` _returnvalue))
  (bind _outhit (`KismetSystemLibrary.LineTraceSingle` :`Start` _returnvalue_2 :`End` (+ _returnvalue_2 (* (`Actor.GetActorForwardVector` _returnvalue) 4000)) :`TraceChannel` "TraceTypeQuery1" :`DrawDebugType` "ForDuration"))
  (`NiagaraFunctionLibrary.SpawnSystemAtLocation` "/Game/ThirdPerson/Blueprints/Explosion.Explosion" (`.ImpactPoint` (`GameplayStatics.BreakHitResult` _outhit))))
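; BP_ItemBase_01 is an item pickup actor that routes its ItemData to the player when its Collision is overlapped.
; ItemType selects the route: inventory items go to the player character's InventoryScan, skill items to AddSkill on the AC_InGameHUD component.
; PickupFeedback then runs, gated by ItemCanBePickedUp, playing a sound, showing an animated W_PickUpFeedback widget and destroying the actor.
; The overlapping actor is never checked; player index 0 always receives the item.
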(event `self.Collision.OnComponentBeginOverlap`
  (params (OverlappedComponent :type "PrimitiveComponent Object Reference") (OtherActor :type "Actor Object Reference") (OtherComp :type "PrimitiveComponent Object Reference") (OtherBodyIndex :type Integer) (bFromSweep :type Boolean) (SweepResult :type "HitResult Structure (by ref)"))
  (bind _returnvalue (`self.GetComponentByClass` (`GameplayStatics.GetPlayerPawn` 0) "/Game/Bps/Inventory/AC_InGameHUD.AC_InGameHUD_C"))
  (switch `/Game/eNUMS/E_ItemType` (`.ItemType_18_5F3DB02940FB839A711C40A677107403` (break `/Game/Bps/Inventory/ST_Items_01` (`self.ItemData`)))
    (:`NewEnumerator0`
      (bind _asbp_third_person_character_inventory (cast `/Game/ThirdPerson/Blueprints/BP_ThirdPersonCharacterInventory` (`GameplayStatics.GetPlayerCharacter` 0)))
      (`/Game/ThirdPerson/Blueprints/BP_ThirdPersonCharacterInventory.InventoryScan` _asbp_third_person_character_inventory (`self.ItemData`))
      (`self.PickupFeedback`))
    (:`NewEnumerator1`
      (`/Engine/EditorBlueprintResources/StandardMacros.IsValid` _returnvalue
        (:`Is Valid`
          (`/Game/Bps/Inventory/AC_InGameHUD.AddSkill` _returnvalue (`self.ItemData`))
          (`self.PickupFeedback`))))))

(event `PickupFeedback`
  (bind _pickupfeedback_ref (`self.PickUpFeedback_REF`))
  (if (`self.ItemCanBePickedUp?`)
    (`GameplayStatics.PlaySoundAtLocation` "/Game/Sounds/332629__treasuresounds__item-pickup.332629__treasuresounds__item-pickup" (`SceneComponent.K2_GetComponentLocation` (`self.DefaultSceneRoot`)) (struct) 1.0 1.0 0.0 null null null null)
    (bind _returnvalue (`|CreateWidget` "/Game/Bps/Inventory/W_PickUpFeedback.W_PickUpFeedback_C"))
    (bind _output_get (set `self.PickUpFeedback_REF` _returnvalue))
    (set `/Game/Bps/Inventory/W_PickUpFeedback.ItemData` (`self.ItemData`) _output_get)
    (`UserWidget.AddToViewport` _pickupfeedback_ref 0)
    (`UserWidget.PlayAnimation` _pickupfeedback_ref (`/Game/Bps/Inventory/W_PickUpFeedback.MoveUp` _pickupfeedback_ref) 0.0 1 "Forward" 1.0 false)
    (`self.K2_DestroyActor`)))

(fn `UserConstructionScript`)
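; BP_Patrol_01 is an actor that moves through a list of patrol points, one point per press of the F key.
; It enables input on BeginPlay, and F plays the PatrolMovement timeline from the start.
; Each update lerps from the actor's current root location, rather than a stored start, toward the current point.
; When the timeline finishes, the point index increments with no wrap or bounds check.
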(event `self.ReceiveBeginPlay`
  (`self.EnableInput` (`GameplayStatics.GetPlayerController` 0)))

(event `Key|F`
  (params (Key :type "Key Structure"))
  (:`Pressed`
    (bind (_direction _newtrack_0) (`Timeline|PatrolMovement` :!via `PlayFromStart`)
      (:`Update`
        (`self.K2_SetActorLocation` (`KismetMathLibrary.VLerp` (`SceneComponent.K2_GetComponentLocation` (`self.DefaultSceneRoot`)) (`self.K2_GetActorLocation` (`|GetArrayItem` (`self.PatrolPoints`) (`self.PatrolPointList`))) _newtrack_0)))
      (:`Finished`
        (set `self.PatrolPointList` (+ (`self.PatrolPointList`) 1))))))

(fn `UserConstructionScript`)